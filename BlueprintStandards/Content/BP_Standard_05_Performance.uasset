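; BP_Standard_05_Performance is a reference Blueprint illustrating coding-standard section 5 on performance, with disconnected example nodes that never run.
; It compares validated gets with separate IsValid checks and favors casting to native classes or the highest parent Blueprint to reduce compile dependencies.
; It also shows interface messages on the player character and a parent-class OnDeath call as the override example.
; The construction script is empty.
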(fn ConstructionScript)