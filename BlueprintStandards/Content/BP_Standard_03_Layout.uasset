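; Style-guide example Blueprint illustrating standard 3 on graph layout, with disconnected, never-run snippets annotated by numbered rule comments.
; Snippets cover Sequence nodes for unrelated flows, reroute nodes, reusing variables, storing function outputs to avoid re-evaluation, and breaking search loops to cache results.
; A function and macro pair contrasts early exit from loops: the function stops at return, while the macro keeps looping and fires both exits.
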(fn ConstructionScript)

(fn GenerateRandomNumber
  (return 0.0))

(fn CalculateDamage)

(fn TakeDamage)

(fn FindBox)

(fn LoopsInsideFunction
  ;[0.3447 0.3333 1] If you execute an output pin in a function, then the loop inside the function will not continue to loop.
  ;
  ; In this example, you would see the log messages for '0' and '1'. The function itself would return only 'TRUE'
  (for (_array_element _array_index) (Utilities|Array|MakeArray false true false)
    (Development|PrintString (Utilities|String|ToString(Integer) _array_index))
    (if _array_element
      (return true)))
  (return false))