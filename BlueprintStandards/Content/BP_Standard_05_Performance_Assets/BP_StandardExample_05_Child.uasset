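; Example child Blueprint that demonstrates overriding parent behavior and responding to Blueprint interface calls, with debug prints standing in for gameplay logic.
; It overrides the parent's OnDeath to print the CausedByFire value and handles EnableWeapons through BPI_Standard_05_Interface by printing the requested state.
; GetWeaponInSlot is a placeholder that prints the slot and returns self, while the construction script only calls the parent's.
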(event EventEnableWeapons
  (params (setEnabled :type Boolean))
  ;[1 1 1] Interface
  (Development|PrintString (Utilities|String|Append "The Child BP does something through the interface BPI_Standard_05_Interface : " (Utilities|String|ToString(Boolean) setEnabled))))

(event EventOnDeath
  (params (causedByFire :type Boolean))
  ;[1 1 1] Override of parent function
  (Development|PrintString (Utilities|String|Append "The Child BP does something different with the CustomBlueprintFunction : " (Utilities|String|ToString(Boolean) causedByFire))))

(fn ConstructionScript
  (|CallParentFunction))

(fn GetWeaponinSlot
  (params (slotToGet :type Integer))
  (Development|PrintString (Utilities|String|ToString(Integer) slotToGet)) ; Example
  (return self))