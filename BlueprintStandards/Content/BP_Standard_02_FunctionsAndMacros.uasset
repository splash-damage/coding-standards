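; Example Blueprint for a coding standard on functions and macros, with commented node snippets that never execute.
; The event graph contrasts bad and good layouts: repeated logic versus DRYFunction or DRYMacro, and unrelated flows split into named functions or Sequence branches.
; It also covers Private, Protected and Public access specifiers and promoting asset references to descriptively named variables.
; Most helper functions are empty stubs; two are unused.
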(fn ConstructionScript)

(fn DRYFunction
  (params (DistanceToTestToObjective :type Float%20%28single-precision%29))
  (if (> DistanceToTestToObjective (Variables|Default|GetMaximumDistanceToObjective))
    (Class|GameplayTasksComponent|RunGameplayTask))
  (Class|VisualLoggerKismetLibrary|LogLocation 0 "0, 0, 0" "" "(R=0.000000,G=0.000000,B=1.000000,A=1.000000)" 1e+01 "VisLogBP"))

(fn GetAIController)

(fn TakeDamage
  (return))

(fn ProtectedFunction)

(fn PrivateFunction)

(fn PublicFunction)

(fn AddValues
  (params (A :type Float%20%28single-precision%29) (B :type Float%20%28single-precision%29))
  (return (+ A B)))

(fn GetCurrentActiveActor
  (return (Utilities|Array|Get(acopy) (Variables|Example|Pure|GetPureExampleArray) (Variables|Example|Pure|GetPureExampleActorToGet))))