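; Reference Blueprint illustrating section 3 of a content standard on graph layout, built as commented examples that never execute.
; The examples show Sequence nodes splitting unrelated flows, storing outputs in variables, reroute nodes, and reusing variables instead of long wires.
; A final example uses a ForEach loop with break to find a named actor and store it.
; Helper functions like CalculateDamage and GenerateRandomNumber are empty or trivial stubs supporting the examples.
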(fn ConstructionScript)

(fn GenerateRandomNumber
  (return 0.0))

(fn CalculateDamage)

(fn TakeDamage)

(fn FindBox)