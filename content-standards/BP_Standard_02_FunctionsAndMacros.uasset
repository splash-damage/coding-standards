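; Example Blueprint for a content standards guide on functions and macros, with commented samples that are not wired to run.
; The event graph contrasts repeated or mixed logic with versions split into functions, macros and Sequence branches.
; It also illustrates Private, Protected and Public access specifiers and promoting asset references to named variables.
; DRYFunction and DRYMacro wrap the same distance-check, gameplay task and logging logic, while most other functions are empty stubs.
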(fn ConstructionScript)

(fn DRYFunction
  (if (> (Variables|Default|GetCurrentDistanceToObjective) (Variables|Default|GetMaximumDistanceToObjective))
    (Class|GameplayTasksComponent|RunGameplayTask))
  (Class|VisualLoggerKismetLibrary|LogLocation 0 "0, 0, 0" "" "(R=0.000000,G=0.000000,B=1.000000,A=1.000000)" 1e+01 "VisLogBP"))

(fn GetAIController)

(fn TakeDamage
  (return))

(fn ProtectedFunction)

(fn PrivateFunction)

(fn PublicFunction)

(fn PureFunction)